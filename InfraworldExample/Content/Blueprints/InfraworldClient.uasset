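; Test actor for the Infraworld gRPC plugin that calls a local HelloService server from mouse input.
; BeginPlay enables input, creates an insecure RPC client to localhost and binds its error, Hello and ServerTime response events, while Tick calls Update on the client.
; Left click sends a Hello request and right click requests the server time; replies and errors print to screen.
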(event `self.ReceiveBeginPlay`
  (`self.EnableInput` (`GameplayStatics.GetPlayerController` 0))
  (bind _returnvalue (`RpcClient.CreateRpcClient` "/Script/InfraworldClientDemo.HelloServiceRpcClient" (make `RpcClientInstantiationParameters` "127.0.0.1" 50051 (`ChannelCredentials.MakeInsecureChannelCredentials`))))
  (bind _output_get (set `self.HelloClient` _returnvalue))
  (add `RpcClient.EventRpcError` _output_get (delegate `ErrorEvent`))
  (add `HelloServiceRpcClient.EventHello` _output_get (delegate `HelloEvent`))
  (add `HelloServiceRpcClient.EventServerTime` _output_get (delegate `CustomEvent_0`)))

(event `self.ReceiveTick`
  (params (DeltaSeconds :type "Float (single-precision)"))
  (`RpcClient.Update` (`self.HelloClient`)))

(event `ErrorEvent`
  (params (Dispatcher :type "RpcClient Object Reference") (Error :type "RpcError Structure (by ref)"))
  (`KismetSystemLibrary.PrintString` Error_ErrorMessage true true (struct :`R` 1.0 :`B` 0.005276 :`A` 1.0) 20.0))

(event `HelloEvent`
  (params (RpcClient :type "HelloServiceRpcClient Object Reference") (Response :type "VizorDemonstration_HelloResponse Structure (by ref)") (Status :type "GrpcStatus Structure"))
  (`KismetSystemLibrary.PrintString` Response_Message true true (struct :`G` 0.66 :`B` 1.0 :`A` 1.0) 10.0))

(event `CustomEvent_0`
  (params (RpcClient :type "HelloServiceRpcClient Object Reference") (Response :type "VizorDemonstration_ServerTimeResponse Structure (by ref)") (Status :type "GrpcStatus Structure"))
  (`KismetSystemLibrary.PrintString` (`KismetStringLibrary.Concat_StrStr` "Server Time:    " (`KismetStringLibrary.Conv_IntToString` Response_Hours) ":" (`KismetStringLibrary.Conv_IntToString` Response_Minutes) ":" (`KismetStringLibrary.Conv_IntToString` Response_Seconds) "     " Response_Timezone "        " Response_Location) true true (struct :`R` 0.871619 :`B` 1.0 :`A` 1.0) 10.0))

(event `Key|LeftMouseButton`
  (params (Key :type "Key Structure"))
  (:`Pressed`
    (`HelloServiceRpcClient.Hello` (`self.HelloClient`) (make `VizorDemonstration_HelloRequest` "Vizor Infraworld Client") (make `GrpcClientContext` _))))

(event `Key|RightMouseButton`
  (params (Key :type "Key Structure"))
  (:`Pressed`
    (`HelloServiceRpcClient.ServerTime` :`self` (`self.HelloClient`) :`Context` (make `GrpcClientContext` _))))

(fn `UserConstructionScript`)